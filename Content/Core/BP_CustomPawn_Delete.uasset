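; BP_CustomPawn_Delete is a player pawn with free directional movement and a spring-arm camera controlled through Enhanced Input.
; Input actions store look and move axes, zeroed on cancel or completion, which Tick feeds into movement and rotation updates.
; Movement follows the normalized camera forward and right vectors, pitch included, setting location directly without sweeping for collision.
; Camera rotation accumulates yaw and clamped pitch, then sets the spring arm's world rotation.
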(event Input|EnhancedActionEvents|EnhancedInputActionIA_CameraMovement
  (params (ActionValue :type Vector%202D%20Structure) (ElapsedSeconds :type Float%20%28double-precision%29) (TriggeredSeconds :type Float%20%28double-precision%29) (InputAction :type Input%20Action%20Object%20Reference :default "/Game/Input/IA_CameraMovement.IA_CameraMovement"))
  (:Triggered
    (Variables|Default|SetLookInput (.y ActionValue))
    (Variables|Default|SetTurnInput (.x ActionValue)))
  (:Canceled
    (Variables|Default|SetLookInput 0.0 :!label _label)
    (Variables|Default|SetTurnInput 0.0))
  (:Completed
    (goto _label)))

(event Input|EnhancedActionEvents|EnhancedInputActionIA_PlayerMovement
  (params (ActionValue :type Vector%202D%20Structure) (ElapsedSeconds :type Float%20%28double-precision%29) (TriggeredSeconds :type Float%20%28double-precision%29) (InputAction :type Input%20Action%20Object%20Reference :default "/Game/Input/IA_PlayerMovement.IA_PlayerMovement"))
  (:Triggered
    (Variables|Default|SetMoveForwardInput (.y ActionValue))
    (Variables|Default|SetMoveRightInput (.x ActionValue)))
  (:Canceled
    (Variables|Default|SetMoveForwardInput 0.0 :!label _label)
    (Variables|Default|SetMoveRightInput 0.0))
  (:Completed
    (goto _label)))

(event EventTick
  (params (DeltaSeconds :type Float%20%28single-precision%29))
  (CallFunction|UpdateMovement DeltaSeconds)
  (CallFunction|UpdateCameraRotation DeltaSeconds))

(fn ConstructionScript)

(fn UpdateMovement
  (params (DeltaTime :type Float%20%28double-precision%29))
  (bind _camerarotation (Variables|Default|GetCameraRotation))
  (bind _output_get (LocalVariables|SetDesiredMoveDirection (Math|Vector|Normalize (+ (* (Math|Vector|GetForwardVector _camerarotation) (Variables|Default|GetMoveForwardInput)) (* (Variables|Default|GetMoveRightInput) (Math|Vector|GetRightVector _camerarotation))))))
  (Transformation|SetActorLocation (+ (Transformation|GetActorLocation) (* (LocalVariables|GetDesiredMoveDirection) DeltaTime (Variables|Default|GetMoveSpeed))) false false))

(fn UpdateCameraRotation
  (params (Delta%20Time :type Float%20%28double-precision%29))
  (bind _output_get (Variables|Default|SetCameraRotation (Math|Rotator|MakeRotator (.Roll (Math|Rotator|BreakRotator (Variables|Default|GetCameraRotation))) (Math|Float|Clamp(Float) (+ (.Pitch (Math|Rotator|BreakRotator (Variables|Default|GetCameraRotation))) (* (Variables|Default|GetLookInput) (Variables|Default|GetTurnSpeed) -1.0 Delta%20Time)) 0.0 85.0) (+ (.Yaw (Math|Rotator|BreakRotator (Variables|Default|GetCameraRotation))) (* (Variables|Default|GetTurnSpeed) Delta%20Time (Variables|Default|GetTurnInput))))))
  (Transformation|SetWorldRotation (Variables|Default|GetSpringArm) _output_get false false))